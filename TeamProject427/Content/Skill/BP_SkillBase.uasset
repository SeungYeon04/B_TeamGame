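; BP_SkillBase is a skill base Blueprint that provides named activation gated by a cooldown.
; ActivateSkill prints a cooldown warning if locked; otherwise it sets the cooldown flag, starts a timer by function name and calls SkillShow.
; SkillShow only prints the skill name, with no gameplay effect.
; When the stored timer fires, CooldownEnd clears the flag; BeginPlay and Tick are empty.
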(fn `Activate Skill`
  (if (`self.bIsOnCooldown`)
    (`KismetSystemLibrary.PrintString` "Cooldown" true true (struct :`R` 1.0 :`G` 0.165041 :`B` 0.214809 :`A` 1.0))
    (else
      (set `self.bIsOnCooldown` true)
      (bind _returnvalue (`KismetSystemLibrary.K2_SetTimer` self "CooldownEnd" (`self.CooldownTime`)))
      (set `self.CooldownTimer` _returnvalue)
      (`self.SkillShow`))))

(fn `CooldownEnd`
  (set `self.bIsOnCooldown` false))

(fn `SkillShow`
  (`KismetSystemLibrary.PrintString` (`self.SkillName`)))